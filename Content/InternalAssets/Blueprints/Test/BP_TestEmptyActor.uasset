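; BP_TestEmptyActor is a test actor that exercises rotation math on its root component through two events.
; DoTurn adds a world rotation built from a quaternion rotation vector, the root's up vector scaled by a constant.
; LockTarget sets the root's world transform with a LookAt toward TargetActor, aiming the X axis with world Z as up.
; An unconnected local yaw rotation and an unused LerpTransform node remain in the graph.
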(event Custom|DoTurn
  (bind _defaultsceneroot (Variables|Default|GetDefaultSceneRoot))
  (Transformation|AddWorldRotation _defaultsceneroot (Class|KismetMathLibrary|QuatRotator (Class|KismetMathLibrary|QuatMakefromRotationVector (* (Math|Vector|GetUpVector _defaultsceneroot) 9e+01))) false false))

(event Custom|LockTarget
  (bind _defaultsceneroot (Variables|Default|GetDefaultSceneRoot))
  (Transformation|SetWorldTransform _defaultsceneroot (Class|KismetAnimationLibrary|Lookat (Transformation|GetWorldTransform _defaultsceneroot) (Transformation|GetActorLocation (Variables|Default|GetTargetActor)) "1.000000,0.000000,0.000000" true "0.000000,0.000000,1.000000" 0.0) false false))

(fn ConstructionScript)